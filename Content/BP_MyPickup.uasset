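; Player-driven pickup vehicle pawn for a race, with throttle, steering, handbrake and camera-look input.
; Input stays disabled until the player controller's RaceStart flag is set; Tick then drives sand spray and engine audio from vehicle speed.
; Tick also detects a flipped, slow car and destroys it if still stuck after a delay, as does the RespawnCar input.
; Destruction calls RespawnVehicle on the controller, which receives the spawn transform at BeginPlay.
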(event `self.ReceiveBeginPlay`
  ;[1 1 1] Disable input when the race has not started yet
  (bind _asb_my_player_controller (cast `/Game/Blueprints/b_MyPlayerController` (`GameplayStatics.GetPlayerController` 0)))
  (bind _output_get (set `self.ControllerReference` _asb_my_player_controller))
  (set `/Game/Blueprints/b_MyPlayerController.RespawnLocation` (`self.GetTransform`) _output_get)
  (`self.DisableInput` (`self.ControllerReference`))
  (`GameplayStatics.SetBaseSoundMix` "/Game/Audio/MySoundMix.MySoundMix"))

(event `self.ReceiveTick`
  (params (DeltaSeconds :type "Float (single-precision)"))
  (bind _controllerreference (`self.ControllerReference`))
  (bind _ns_sandspray (`self.NS_SandSpray`))
  ;[1 1 1] Enable Input if Race has started
  (if (`/Game/Blueprints/b_MyPlayerController.RaceStart` _controllerreference)
    (`self.EnableInput` _controllerreference)
    ;[1 1 1] Activate/Deactivate sand particles depending on velocity
    (if (> (`KismetMathLibrary.VSize` (`self.GetVelocity`)) 500.0)
      (`ActorComponent.Activate` _ns_sandspray false)
      (else
        (`ActorComponent.Deactivate` _ns_sandspray)))
    ;[1 1 1] Fade in/out engine sounds based on velocity
    (`AudioComponent.SetFloatParameter` (`self.Engine_Noise`) "Velocity" (`KismetMathLibrary.Abs` (`WheeledVehicleMovementComponent.GetForwardSpeed` (`self.VehicleMovement`))))
    ;[1 1 1] Checking if Player has flipped the car and is stuck, if so call Respawn Vehicle in My Player Controller
    (bind _isplayerstuck (`self.RespawnCheck`))
    (if _isplayerstuck
      (`KismetSystemLibrary.Delay` 4.0)
      (bind _isplayerstuck_2 (`self.RespawnCheck`))
      (if _isplayerstuck_2
        (`self.K2_DestroyActor`)))))

(event `self.ReceiveDestroyed`
  ;[1 1 1] Checking if Player has flipped the car and is stuck, if so call Respawn Vehicle in My Player Controller
  (`/Game/Blueprints/b_MyPlayerController.RespawnVehicle` (`self.ControllerReference`)))

(event `InputAction|RespawnCar`
  (params (Key :type "Key Structure"))
  ;[1 1 1] Destroy Car when Backspace pressed
  (:`Pressed`
    (`/Engine/EditorBlueprintResources/StandardMacros.DoOnce` false
      (:`Completed`
        (`self.K2_DestroyActor`)))))

(event `InputAxis|MoveForward`
  (params (AxisValue :type "Float (single-precision)"))
  ;[1 1 1] Vehicle Movement
  (`WheeledVehicleMovementComponent.SetThrottleInput` (`self.VehicleMovement`) AxisValue))

(event `InputAxis|MoveRight`
  (params (AxisValue :type "Float (single-precision)"))
  ;[1 1 1] Vehicle Movement
  (`WheeledVehicleMovementComponent.SetSteeringInput` (`self.VehicleMovement`) AxisValue))

(event `InputAction|Handbrake`
  (params (Key :type "Key Structure"))
  (bind _vehiclemovement (`self.VehicleMovement`))
  ;[1 1 1] Vehicle Movement
  (:`Pressed`
    (`WheeledVehicleMovementComponent.SetHandbrakeInput` _vehiclemovement true))
  (:`Released`
    (`WheeledVehicleMovementComponent.SetHandbrakeInput` _vehiclemovement false)))

(event `InputAxis|LookUp`
  (params (AxisValue :type "Float (single-precision)"))
  ;[1 1 1] Vehicle Movement
  (`self.AddControllerPitchInput` (* AxisValue -1.0)))

(event `InputAxis|LookRight`
  (params (AxisValue :type "Float (single-precision)"))
  ;[1 1 1] Vehicle Movement
  (`self.AddControllerYawInput` AxisValue))

(fn `RespawnCheck`
  (returns (IsPlayerStuck :type Boolean))
  ;[1 1 1] Check if player not moving and upside down
  (if (and (< (`KismetMathLibrary.Dot_VectorVector` (`self.GetActorUpVector`) (0.0 0.0 1.0)) 0.5) (< (`WheeledVehicleMovementComponent.GetForwardSpeed` (`self.VehicleMovement`)) 0.5))
    (set `self.isStuck` true)
    (else
      (set `self.isStuck` false)))
  (return (`self.isStuck`)))

(fn `UserConstructionScript`)